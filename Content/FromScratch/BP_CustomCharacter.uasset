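; BP_CustomCharacter is a player character driven by Enhanced Input actions for move, look, sprint, jump and attack.
; Movement follows the full control rotation, with input X as forward and Y as right, while look feeds controller yaw and pitch.
; Sprint toggles max walk speed on input completion.
; Jump, also on completion, uses delays around Jump and StopJumping while flagging IsJumping, and attack plays a montage.
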(event `EnhancedInput|/Game/FromScratch/IA_Move_Custom`
  (params (ActionValue :type "Vector2D Structure") (ElapsedSeconds :type "Float (double-precision)") (TriggeredSeconds :type "Float (double-precision)") (InputAction :type "InputAction Object Reference" :default "/Game/FromScratch/IA_Move_Custom.IA_Move_Custom"))
  (:`Triggered`
    (`self.AddMovementInput` (`KismetMathLibrary.GetForwardVector` (`self.GetControlRotation`)) ActionValue_X)
    (`self.AddMovementInput` (`KismetMathLibrary.GetRightVector` (`self.GetControlRotation`)) ActionValue_Y)))

(event `EnhancedInput|/Game/FromScratch/IA_Look_Custom`
  (params (ActionValue :type "Vector2D Structure") (ElapsedSeconds :type "Float (double-precision)") (TriggeredSeconds :type "Float (double-precision)") (InputAction :type "InputAction Object Reference" :default "/Game/FromScratch/IA_Look_Custom.IA_Look_Custom"))
  (:`Triggered`
    (`self.AddControllerYawInput` ActionValue_X)
    (`self.AddControllerPitchInput` ActionValue_Y)))

(event `EnhancedInput|/Game/FromScratch/IA_Sprint_Custom`
  (params (ActionValue :type Boolean) (ElapsedSeconds :type "Float (double-precision)") (TriggeredSeconds :type "Float (double-precision)") (InputAction :type "InputAction Object Reference" :default "/Game/FromScratch/IA_Sprint_Custom.IA_Sprint_Custom"))
  (:`Completed`
    (if (`self.Is Sprinting`)
      (set `CharacterMovementComponent.MaxWalkSpeed` 300.0 (`self.CharacterMovement`))
      (set `self.Is Sprinting` false)
      (else
        (set `CharacterMovementComponent.MaxWalkSpeed` 600.0 (`self.CharacterMovement`))
        (set `self.Is Sprinting` true)))))

(event `EnhancedInput|/Game/FromScratch/IA_Jump_Custom`
  (params (ActionValue :type Boolean) (ElapsedSeconds :type "Float (double-precision)") (TriggeredSeconds :type "Float (double-precision)") (InputAction :type "InputAction Object Reference" :default "/Game/FromScratch/IA_Jump_Custom.IA_Jump_Custom"))
  (:`Completed`
    (set `self.Is Jumping` true)
    (`KismetSystemLibrary.Delay` 0.5)
    (`self.Jump`)
    (`KismetSystemLibrary.Delay` 0.2)
    (`self.StopJumping`)
    (set `self.Is Jumping` false)))

(event `EnhancedInput|/Game/FromScratch/IA_Attack_Custom`
  (params (ActionValue :type Boolean) (ElapsedSeconds :type "Float (double-precision)") (TriggeredSeconds :type "Float (double-precision)") (InputAction :type "InputAction Object Reference" :default "/Game/FromScratch/IA_Attack_Custom.IA_Attack_Custom"))
  (:`Completed`
    (`self.PlayAnimMontage` "/Game/Characters/Mannequins/Anims/Unarmed/Attack/AM_Attack_01.AM_Attack_01")))

(fn `UserConstructionScript`)